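; Treasure chest actor demonstrating network relevancy and RepNotify replication, with a ground ring scaled from its net cull distance.
; On first box overlap, the server sets IsChestOpened and calls ChestTouchedMulticast.
; The RepNotify rotates the lid open as lasting state, while the multicast event spawns the one-off gold burst on the treasure pile.
; An alternative OnChestTouched path on both authority and remote is left unconnected.
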(event OnComponentBeginOverlap(Box)
  (params (OverlappedComponent :type Primitive%20Component%20Object%20Reference) (OtherActor :type Actor%20Object%20Reference) (OtherComp :type Primitive%20Component%20Object%20Reference) (OtherBodyIndex :type Integer) (bFromSweep :type Boolean) (SweepResult :type Hit%20Result%20Structure%20%28by%20ref%29))
  ;[1 1 1 1 25] 오버랩 되면 박스 여는 노드
  (Networking|SwitchHasAuthority
    (:Authority
      (Utilities|FlowControl|DoOnce false
        (:Completed
          (Variables|Default|SetIsChestOpened true)
          (CallFunction|ChestTouchedMulticast))))))

(event Custom|ChestTouchedMulticast
  ;[1 1 1 1 25] 오버랩 되면 박스 여는 노드
  (CallFunction|PlayGoldFX))

(event EventBeginPlay
  (bind _netculldistancesquared (Variables|Default|GetNetCullDistanceSquared))
  (bind _returnvalue (Math|Float|Sqrt _netculldistancesquared))
  (bind _returnvalue_2 (/ _returnvalue 3e+01))
  ;[1 1 1 1 25] 링 크기를 바꾸는 노드
  (Transformation|SetWorldScale3D (Variables|Default|GetSM_Radius_Ring) (Math|Vector|MakeVector _returnvalue_2 _returnvalue_2 1.0)))

(event Collision|EventActorBeginOverlap
  (params (OtherActor :type Actor%20Object%20Reference)))

(event EventTick
  (params (DeltaSeconds :type Float%20%28single-precision%29)))

(fn ConstructionScript)

(fn OpenChest
  ;[1 1 1] 이벤트 발생시 y축으로 180도 돈다
  (Transformation|SetRelativeRotation (Variables|Default|GetSM_Chest_Lid) "180.000000,0.000000,0.000000" false false))

(fn PlayGoldFX
  ;[1 1 1] 이벤트 발생시 이미터 실행
  (Effects|SpawnEmitterAttached "/Game/ExampleContent/NetworkFeatures/Effects/P_Treasure_Burst.P_Treasure_Burst" (Variables|Default|GetSM_Treasure_Pile) "None" "0.000000,0.000000,10.000000"))

(fn OnChestTouched
  (CallFunction|OpenChest)
  (CallFunction|PlayGoldFX))

(fn OnRepIsChestOpened
  ;[1 1 1] 오픈
  (if (Variables|Default|GetIsChestOpened)
    (CallFunction|OpenChest)))