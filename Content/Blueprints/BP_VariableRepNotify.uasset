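; Traffic light actor that demonstrates a replicated RepNotify variable driving its light state.
; Only the authority changes StreetlightScalar, through an endless delayed yellow, green, red loop with a random wait on red.
; Box overlaps also set it, red on begin and green on end, without pausing the loop.
; OnRep_StreetlightScalar writes the value into a dynamic material instance created on the mesh in the construction script.
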(event OnComponentBeginOverlap(Box)
  (params (OverlappedComponent :type Primitive%20Component%20Object%20Reference) (OtherActor :type Actor%20Object%20Reference) (OtherComp :type Primitive%20Component%20Object%20Reference) (OtherBodyIndex :type Integer) (bFromSweep :type Boolean) (SweepResult :type Hit%20Result%20Structure%20%28by%20ref%29))
  (Networking|SwitchHasAuthority
    (:Authority
      (Variables|Default|SetStreetlightScalar (Variables|Default|GetRedScalar)))))

(event OnComponentEndOverlap(Box)
  (params (OverlappedComponent :type Primitive%20Component%20Object%20Reference) (OtherActor :type Actor%20Object%20Reference) (OtherComp :type Primitive%20Component%20Object%20Reference) (OtherBodyIndex :type Integer))
  (Networking|SwitchHasAuthority
    (:Authority
      (Variables|Default|SetStreetlightScalar (Variables|Default|GetGreenScalar)))))

(event EventBeginPlay
  (Utilities|FlowControl|Sequence
    (:then_0
      (Networking|SwitchHasAuthority :!label _label
        (:Authority
          (Utilities|FlowControl|Delay (Math|Random|RandomFloatinRange 2.0 5.0))
          (Variables|Default|SetStreetlightScalar (Variables|Default|GetYellowScalar))
          (Utilities|FlowControl|Delay 1.0)
          (Variables|Default|SetStreetlightScalar (Variables|Default|GetGreenScalar))
          (Utilities|FlowControl|Delay 1.0)
          (Variables|Default|SetStreetlightScalar (Variables|Default|GetRedScalar))
          (goto _label))))))

(event Collision|EventActorBeginOverlap
  (params (OtherActor :type Actor%20Object%20Reference)))

(event EventTick
  (params (DeltaSeconds :type Float%20%28single-precision%29)))

(fn ConstructionScript
  (bind _returnvalue (Rendering|Material|CreateDynamicMaterialInstance (Variables|Default|GetSM_Traffic_Light) 1 0 "None" :!class /Script/Engine.PrimitiveComponent))
  (Variables|Default|SetMI_Light _returnvalue))

(fn OnRepStreetlightScalar
  (Rendering|Material|SetScalarParameterValue (Variables|Default|GetMI_Light) (Variables|Default|GetStreetlightScalarParamName) (Variables|Default|GetStreetlightScalar) :!class /Script/Engine.MaterialInstanceDynamic))