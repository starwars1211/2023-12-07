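; BP_VariableReplication is a demo actor, named for variable replication, that shows a continuously draining Health value on a text render.
; On BeginPlay, only the authority fills Health to maximum and starts a looping timer that calls UpdateHealth.
; Each timer call subtracts a set amount and resets Health to maximum at zero or below.
; Tick writes the current Health to the TextRender without an authority check.
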(event EventBeginPlay
  (Networking|SwitchHasAuthority
    (:Authority
      (CallFunction|InitializeHealth)
      (Utilities|Time|SetTimerbyFunctionName 0 "UpdateHealth" (Variables|Default|GetHelthEcrementTime) true))))

(event Collision|EventActorBeginOverlap
  (params (OtherActor :type Actor%20Object%20Reference)))

(event EventTick
  (params (DeltaSeconds :type Float%20%28single-precision%29))
  (bind _textrender (Variables|Default|GetTextRender))
  (Utilities|IsValid _textrender
    (:Is%20Valid
      (Rendering|Components|TextRender|SetText _textrender (Utilities|Text|ToText(String) (Utilities|String|Append "Health" (Utilities|String|ToString(Integer) (Variables|Default|GetHealth))))))))

(fn ConstructionScript)

(fn InitializeHealth
  (Variables|Default|SetHealth (Variables|Default|GetMaxHealth)))

(fn UpdateHealth
  (bind _output_get (Variables|Default|SetHealth (- (Variables|Default|GetHealth) (Variables|Default|GetHelthDecrementAmt))))
  (if (<= _output_get 0)
    (CallFunction|InitializeHealth)))