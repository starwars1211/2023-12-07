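; BP_Color is a cube actor that changes color with repeated input and then destroys its cube.
; BeginPlay creates a dynamic material instance on the cube.
; Each press of the 1 key raises a counter, sound pitch and Color parameter, and attaches a particle emitter.
; At five presses it spawns and immediately destroys an emitter, then removes the cube; the cube's OnClicked event is empty.
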(event OnClicked(Cube)
  (params (TouchedComponent :type Primitive%20Component%20Object%20Reference) (ButtonPressed :type Key%20Structure :default "None"))
  ;[1 1 1 1 50] 클릭이용해서 색깔 체인지 후 디스트로이
)

(event Custom|1
  ;[1 1 1 1 50] 클릭이용해서 색깔 체인지 후 디스트로이
  (bind _output_get (Variables|Default|SetClick (+ (Variables|Default|GetClick) 1)))
  (bind _output_get_2 (Variables|Default|SetPitchChange (+ (Variables|Default|GetPitchChange) 0.2)))
  (Audio|PlaySound2D "/Engine/EditorSounds/Notifications/CompileSuccess.CompileSuccess" 1.0 _output_get_2 0.0 0 0)
  (bind _output_get_3 (Variables|Default|SetColorChange (+ (Variables|Default|GetColorChange) 5e+01)))
  (Rendering|Material|SetVectorParameterValue (Variables|Default|GetMaterialInstance) "Color" (Utilities|Struct|MakeLinearColor _output_get_3 _output_get_3 _output_get_3 0.1) :!class /Script/Engine.MaterialInstanceDynamic)
  (Effects|SpawnEmitterAttached "/Engine/Tutorial/SubEditors/TutorialAssets/TutorialParticleSystem.TutorialParticleSystem" (Variables|Default|GetCube) "None" (Math|Conversions|ToVector(Float) _output_get_3))
  (if (>= _output_get 5)
    (bind _returnvalue (Effects|SpawnEmitteratLocation "/Engine/Tutorial/SubEditors/TutorialAssets/TutorialParticleSystem.TutorialParticleSystem" (Transformation|GetWorldLocation (Variables|Default|GetCube))))
    (Components|DestroyComponent _returnvalue)
    (Components|DestroyComponent (Variables|Default|GetCube))
    (Audio|PlaySound2D 0 1.0 1.0 0.0 0 0)))

(event EventBeginPlay
  (bind _returnvalue (Rendering|Material|CreateDynamicMaterialInstance (Variables|Default|GetCube) 0 0 "None" :!class /Script/Engine.PrimitiveComponent))
  (Variables|Default|SetMaterialInstance _returnvalue))

(event Collision|EventActorBeginOverlap
  (params (OtherActor :type Actor%20Object%20Reference)))

(event EventTick
  (params (DeltaSeconds :type Float%20%28single-precision%29)))

(fn ConstructionScript)